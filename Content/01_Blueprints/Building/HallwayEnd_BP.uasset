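; HallwayEnd_BP is a hallway end building piece that randomly places a room on one of its two child actor slots.
; On BeginPlay a weighted 50/50 roll assigns RoomGeneration to one slot and Wall to the other, then sets the spawned room's Live flag to false.
; The construction script scales the static mesh from Length, Width and Height.
; Leftover unconnected nodes for an extra roll and an all-wall layout never run.
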(event EventBeginPlay
  (bind _childactor1 (Variables|Default|GetChildActor1))
  (bind _childactor (Variables|Default|GetChildActor))
  (if (Math|Random|RandomBoolwithWeight 0.5)
    (ChildActorComponent|SetChildActorClass (Variables|Default|GetChildActor) "/Game/01_Blueprints/Building/Wall.Wall_C")
    (ChildActorComponent|SetChildActorClass _childactor1 "/Game/01_Blueprints/Building/RoomGeneration.RoomGeneration_C")
    (bind _asroom_generation (Utilities|Casting|CastToRoomGeneration (Variables|/Script/Engine.ChildActorComponent|GetChildActor _childactor1)))
    (Variables|/Game/01_Blueprints/Building/RoomGeneration.RoomGeneration_C|SetLive _asroom_generation false)
    (else
      (ChildActorComponent|SetChildActorClass (Variables|Default|GetChildActor1) "/Game/01_Blueprints/Building/Wall.Wall_C")
      (ChildActorComponent|SetChildActorClass _childactor "/Game/01_Blueprints/Building/RoomGeneration.RoomGeneration_C")
      (bind _asroom_generation_2 (Utilities|Casting|CastToRoomGeneration (Variables|/Script/Engine.ChildActorComponent|GetChildActor _childactor)))
      (Variables|/Game/01_Blueprints/Building/RoomGeneration.RoomGeneration_C|SetLive _asroom_generation_2 false))))

(fn ConstructionScript
  (Transformation|SetWorldScale3D (Variables|Default|GetStaticMesh) (Math|Vector|MakeVector (Variables|Default|GetLength) (Variables|Default|GetWidth) (Variables|Default|GetHeight))))