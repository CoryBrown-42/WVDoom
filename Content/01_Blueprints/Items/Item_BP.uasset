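; Item_BP is a pickup item actor whose mesh is set from its ItemInfo at construction.
; Pickup stops physics and plays a timeline that pulls the mesh toward a point above the player's head socket while squashing it horizontally.
; When the timeline finishes, it adds ItemInfo to the player's inventory, plays the pickup sound and destroys itself.
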(event EventBeginPlay)

(event EventPickup
  (params (Player :type Player%20BP%20Object%20Reference))
  (bind _iteminfo (Variables|Info|GetItemInfo))
  (Physics|SetSimulatePhysics (Variables|Default|GetMesh) false)
  (bind _newtrack_0 (Timeline|Lerp PlayFromStart)
    (:Update
      (CallFunction|AddtheJuice (Variables|/Script/Engine.Character|GetMesh Player) _newtrack_0))
    (:Finished
      (Utilities|Array|Add (.inventory (Variables|/Game/01_Blueprints/Player/Player_BP.Player_BP_C|GetPlayerInfo Player)) _iteminfo)
      (Audio|PlaySound2D (.PickupSound (Utilities|Struct|BreakItemInfo _iteminfo)) 1.0 1.0 0.0 0 0)
      (Actor|DestroyActor))))

(fn ConstructionScript
  (Components|StaticMesh|SetStaticMesh (Variables|Default|GetMesh) (.mesh (Variables|Info|GetItemInfo))))

(fn AddtheJuice
  (params (Player :type Scene%20Component%20Object%20Reference) (Lerp :type Float%20%28single-precision%29))
  (bind _mesh (Variables|Default|GetMesh))
  (Transformation|SetWorldLocation _mesh (Math|Vector|Lerp(Vector) (Transformation|GetWorldLocation _mesh) (+ (Transformation|GetSocketLocation Player "head") "0, 0,30.000000") Lerp) false true)
  (Transformation|SetWorldScale3D _mesh (Math|Vector|Lerp(Vector) "1.000000,1.000000,1.000000" "0.100000,0.100000,1.000000" Lerp)))